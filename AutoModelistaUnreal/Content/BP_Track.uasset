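; Track actor that holds a racing line spline and gives the first BP_Car it finds a point to steer toward.
; Each tick it shifts the car's location by Distance against the spline's local right vector, then snaps that point to the line as the car's SteeringDirection.
; A sphere marks the target, and an arrow at the car's closest spline point shows that reversed right-vector direction.
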(event EventTick
  (params (DeltaSeconds :type Float%20%28single-precision%29))
  (bind _racingline (Variables|Default|GetRacingLine))
  (bind _car (Variables|Default|GetCar))
  (bind _racingline_2 (Variables|Default|GetRacingLine))
  (bind _returnvalue (Transformation|GetActorLocation _car))
  (bind _returnvalue_2 (Class|SplineComponent|FindRightVectorClosesttoWorldLocation _racingline_2 _returnvalue "Local"))
  (bind _returnvalue_3 (Math|Rotator|MakeRotationfromAxes _returnvalue_2 "0, 0, 0" "0, 0, 0"))
  (bind (_roll _pitch _yaw) (Math|Rotator|BreakRotator _returnvalue_3))
  (bind _output_get (Variables|/Game/CarPawn/BP_Car.BP_Car_C|SetSteeringDirection (Variables|Default|GetCar) (Spline|FindLocationClosesttoWorldLocation _racingline (- _returnvalue (* (Math|Vector|GetForwardVector _returnvalue_3) (Variables|Default|GetDistance))) "World")))
  (Transformation|SetWorldLocation (Variables|Default|GetSphere) _output_get false false)
  (Transformation|SetWorldLocationAndRotation (Variables|Default|GetArrow) (Spline|FindLocationClosesttoWorldLocation _racingline _returnvalue "World") (Math|Rotator|MakeRotator _roll _pitch (- _yaw 1.8e+02)) false false))

(event EventBeginPlay
  (bind _returnvalue (Actor|GetActorOfClass "/Game/CarPawn/BP_Car.BP_Car_C"))
  (Variables|Default|SetCar _returnvalue))

(fn ConstructionScript)