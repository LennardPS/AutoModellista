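; BP_TimingGates is a lap timer that finds BP_Car at BeginPlay and prints the current lap time every frame.
; While IsLapStarted is true, Tick counts tenths into seconds through a 0.1-second Delay, so accuracy depends on frame rate.
; EndLap resets the count when the car overlaps StartGate.
; StartLap is empty, its only call is unreachable, and nothing here sets IsLapStarted.
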(event Custom|StartLap)

(event Custom|EndLap
  (if (Collision|IsOverlappingActor (Variables|Default|GetStartGate) (Variables|Default|GetCarRef) :!class /Script/Engine.PrimitiveComponent)
    (Variables|Default|SetTenthOfSecond 0)
    (Variables|Default|SetSeconds 0)))

(event EventBeginPlay
  (bind _returnvalue (Actor|GetActorOfClass "/Game/CarPawn/BP_Car.BP_Car_C"))
  (Variables|Default|SetCarRef _returnvalue))

(event EventTick
  (params (DeltaSeconds :type Float%20%28single-precision%29))
  (Utilities|FlowControl|Sequence
    (:then_0
      (if (Variables|Default|GetIsLapStarted)
        (Utilities|FlowControl|Delay 0.1)
        (Variables|Default|SetTenthOfSecond (+ (Variables|Default|GetTenthOfSecond) 1))
        (if (>= (Variables|Default|GetTenthOfSecond) 10)
          (Variables|Default|SetTenthOfSecond 0)
          (Variables|Default|SetSeconds (+ (Variables|Default|GetSeconds) 1)))))
    (:then_1
      (Development|PrintString (Utilities|String|Append "Current Lap " (Utilities|String|Append (Utilities|String|Append (Utilities|String|ToString(Integer) (Variables|Default|GetSeconds)) ".") (Utilities|String|ToString(Integer) (Variables|Default|GetTenthOfSecond)))) true true "(R=0.000000,G=0.660000,B=1.000000,A=1.000000)" DeltaSeconds))))

(fn ConstructionScript)