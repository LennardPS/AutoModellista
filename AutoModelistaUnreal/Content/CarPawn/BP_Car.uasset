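; BP_Car is a physics-driven car pawn with keyboard, touch and mouse input.
; Held inputs run Timelines whose updates apply drive or reverse force to the rear wheels and yaw torque to the body.
; Tick also applies steering torque scaled by SteeringCalc, whose mapping logic is unwired, and counters sideways slip with a Grip-scaled lateral force.
; Per-frame debug line traces visualize velocity, steering, forward direction and drift.
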(event Custom|WirelessTick
  (Class|PrimitiveComponent|AddTorqueinDegrees (Variables|Default|GetBody) (Math|Vector|MakeVector 0.0 0.0 (* (Variables|Default|GetTurnForce) (Utilities|SteeringCalc))) "None" false))

(event EventTick
  (params (DeltaSeconds :type Float%20%28single-precision%29))
  (bind _grip (Variables|Default|GetGrip))
  (bind _body (Variables|Default|GetBody))
  (CallFunction|WirelessTick)
  (bind _returnvalue (Physics|GetPhysicsLinearVelocity (Variables|Default|GetBody) "None"))
  (Variables|Default|SetLinearVelocity _returnvalue)
  (Variables|Default|SetDriftOffset (Math|Vector|DotProduct (Math|Vector|Normalize (Variables|Default|GetLinearVelocity)) (Math|Vector|GetRightVector (Variables|Default|GetBody))))
  (|DirectionOfTravelTrace)
  (|SteeringDirectionTrace)
  (|ForwardDirectionTrace)
  (|LateralFrictionTrace)
  (Physics|AddForce _body (* (* (Math|Vector|GetRightVector _body) (* (Variables|Default|GetDriftOffset) -1.0)) (Math|Vector|MakeVector _grip _grip _grip)) "None" false)
  (Development|PrintString "Hello" true true "(R=0.000000,G=0.660000,B=1.000000,A=1.000000)" DeltaSeconds))

(event Input|MouseEvents|RightMouseButton
  (params (Key :type Key%20Structure :default "None"))
  (:Pressed
    (Timeline|Timeline_1 PlayFromStart
      (:Update
        (Physics|AddForce (Variables|Default|GetBL_Wheel) (* (* (Math|Vector|GetForwardVector (Variables|Default|GetBody)) (Variables|Default|GetForce)) "-1.000000,-1.000000,-1.000000") "None" false))))
  (:Released
    (Timeline|Timeline_1 Stop)))

(event Input|KeyboardEvents|A
  (params (Key :type Key%20Structure :default "None"))
  (:Pressed
    (Timeline|Timeline_2 PlayFromStart
      (:Update
        (Class|PrimitiveComponent|AddTorqueinDegrees (Variables|Default|GetBody) (Math|Vector|MakeVector 0.0 0.0 (* (Variables|Default|GetTurnForce) (Utilities|SteeringCalc))) "None" false))))
  (:Released
    (Timeline|Timeline_2 Stop)))

(event Input|KeyboardEvents|Right
  (params (Key :type Key%20Structure :default "None"))
  (:Pressed
    (Timeline|Timeline_3 PlayFromStart
      (:Update
        (Class|PrimitiveComponent|AddTorqueinDegrees (Variables|Default|GetBody) (Math|Vector|MakeVector 0.0 0.0 (Variables|Default|GetTurnForce)) "None" false))))
  (:Released
    (Timeline|Timeline_3 Stop)))

(event Input|KeyboardEvents|Left
  (params (Key :type Key%20Structure :default "None"))
  (:Pressed
    (Timeline|Timeline_2 PlayFromStart
      (:Update
        (Class|PrimitiveComponent|AddTorqueinDegrees (Variables|Default|GetBody) (Math|Vector|MakeVector 0.0 0.0 (* (Variables|Default|GetTurnForce) (Utilities|SteeringCalc))) "None" false))))
  (:Released
    (Timeline|Timeline_2 Stop)))

(event Input|KeyboardEvents|D
  (params (Key :type Key%20Structure :default "None"))
  (:Pressed
    (Timeline|Timeline_3 PlayFromStart
      (:Update
        (Class|PrimitiveComponent|AddTorqueinDegrees (Variables|Default|GetBody) (Math|Vector|MakeVector 0.0 0.0 (Variables|Default|GetTurnForce)) "None" false))))
  (:Released
    (Timeline|Timeline_3 Stop)))

(event Input|TouchEvents|InputTouch
  (params (Location :type Vector) (FingerIndex :type ETouchIndex%20Enum))
  (:Pressed
    (Timeline|Timeline_0 PlayFromStart
      (:Update
        (Physics|AddForce (Variables|Default|GetBL_Wheel) (* (Math|Vector|GetForwardVector (Variables|Default|GetBody)) (Variables|Default|GetForce)) "None" false))))
  (:Released
    (Timeline|Timeline_0 Stop)))

(fn ConstructionScript)