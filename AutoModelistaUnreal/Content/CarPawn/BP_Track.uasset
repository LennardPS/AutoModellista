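; Track actor with a spline racing line that feeds a steering target to the BP_Car it finds at BeginPlay.
; Construction sets the loop state and measures the spline; BeginPlay lays non-colliding meshes along it at arrow spacing.
; Each Tick it offsets the car's location along the line's direction, scaled by velocity input magnitude, snaps that to the spline as SteeringDirection, and moves a sphere there.
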(event EventTick
  (params (DeltaSeconds :type Float%20%28single-precision%29))
  (bind _racingline (Variables|Default|GetRacingLine))
  (bind _car (Variables|Default|GetCar))
  (bind _returnvalue (Transformation|GetActorLocation _car))
  (bind _returnvalue_2 (Class|SplineComponent|FindRightVectorClosesttoWorldLocation _racingline _returnvalue "Local"))
  (bind _returnvalue_3 (Math|Rotator|MakeRotationfromAxes _returnvalue_2 "0, 0, 0" "0, 0, 0"))
  (bind (_roll _pitch _yaw) (Math|Rotator|BreakRotator _returnvalue_3))
  (bind _output_get (Variables|/Game/CarPawn/BP_Car.BP_Car_C|SetSteeringDirection (Variables|Default|GetCar) (Spline|FindLocationClosesttoWorldLocation (Variables|Default|GetRacingLine) (- _returnvalue (* (Math|Vector|GetForwardVector (Math|Rotator|MakeRotator _roll _pitch (- _yaw 9e+01))) (* (Variables|Default|GetDistance) (Math|Float|MapRangeUnclamped (Math|Vector|VectorLength (Variables|Default|GetCarVelocityInput)) 0.0 3e+03 1.0 4.0)))) "World")))
  (Transformation|SetWorldLocation (Variables|Default|GetSphere) _output_get false false))

(event EventBeginPlay
  (bind _racingline (Variables|Default|GetRacingLine))
  (bind _returnvalue (Actor|GetActorOfClass "/Game/CarPawn/BP_Car.BP_Car_C"))
  (Variables|Default|SetCar _returnvalue)
  (for _index (range 0 (Math|Float|Floor (/ (Variables|Default|GetTrackLength) (Variables|Default|GetArrowSpacing))))
    (bind _returnvalue_2 (AddComponent|AddStaticMeshComponent false (Math|Transform|MakeTransform (Spline|GetLocationatDistanceAlongSpline _racingline (* _index (Variables|Default|GetArrowSpacing)) "Local") (Spline|GetRotationatDistanceAlongSpline _racingline (* _index (Variables|Default|GetArrowSpacing)) "Local") "1,1,1")))
    (Collision|SetCollisionEnabled _returnvalue_2 "NoCollision")))

(fn ConstructionScript
  (Utilities|FlowControl|Sequence
    (:then_0
      (Spline|SetClosedLoop (Variables|Default|GetRacingLine) (Variables|Default|GetIsClosedLoop) true))
    (:then_1
      (Variables|Default|SetTrackLength (Spline|GetSplineLength (Variables|Default|GetRacingLine))))))