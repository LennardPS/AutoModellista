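; Interactable actor that spins its Cube around the yaw axis as a click is held and dragged horizontally.
; IsClickHold receives screen X and sets the cube's yaw to the offset from a starting X stored through a DoOnce, printing that offset.
; BeginPlay creates a dynamic material on the cube, not used further, and enables player input.
; IsClicked is an empty stub, while IsReleased leads into the DoOnce.
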(event EventIsReleased
  (params (ScreenX :type Float%20%28single-precision%29) (ScreenY :type Float%20%28single-precision%29))
  (Utilities|FlowControl|DoOnce false
    (:Completed
      (Variables|Default|SetHoldInitialX (stale EventIsClickHold ScreenX)))))

(event EventIsClicked
  (params (ScreenX :type Float%20%28single-precision%29) (ScreenY :type Float%20%28single-precision%29)))

(event EventBeginPlay
  (Rendering|Material|CreateDynamicMaterialInstance (Variables|Default|GetCube) 0 0 "Colour" :!class /Script/Engine.PrimitiveComponent)
  (Input|EnableInput (Game|GetPlayerController 0)))

(event EventIsClickHold
  (params (ScreenX :type Float%20%28single-precision%29) (ScreenY :type Float%20%28single-precision%29))
  (Utilities|FlowControl|Sequence
    (:then_0
      (Utilities|FlowControl|DoOnce false
        (:Completed
          (Variables|Default|SetHoldInitialX ScreenX))))
    (:then_1
      (Variables|Default|SetHoldCurrentX ScreenX)
      (Development|PrintString (Utilities|String|ToString(Float) (- (Variables|Default|GetHoldInitialX) (Variables|Default|GetHoldCurrentX))))
      (Transformation|SetRelativeRotation (Variables|Default|GetCube) (Math|Rotator|MakeRotator 0.0 0.0 (- (Variables|Default|GetHoldInitialX) (Variables|Default|GetHoldCurrentX))) false false))))

(fn ConstructionScript)