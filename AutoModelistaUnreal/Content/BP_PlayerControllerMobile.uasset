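; Mobile touch input handler that turns taps, holds and releases into messages on world objects.
; The M_Hold macro uses a short retriggerable delay and two gates to tell taps from holds, always signalling release.
; Taps message the WorldDynamic actor under the cursor; holds cache it and a timeline streams the moving touch X until release.
; Only screen X is passed, with Y always zero.
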(event Custom|Click
  (params (X :type Float%20%28single-precision%29) (Y :type Float%20%28single-precision%29))
  (bind _returnvalue (Game|GetPlayerController 0))
  (bind _array (Utilities|Array|MakeArray "ObjectTypeQuery2"))
  (bind _hitresult (Class|PlayerController|GetHitResultUnderCursorforObjects _returnvalue _array true))
  (bind (_bblockinghit _binitialoverlap _time _distance _location _impactpoint _normal _impactnormal _physmat _hitactor) (Collision|BreakHitResult _hitresult))
  (if _bblockinghit
    _
    (else
      _))
  (Class|BPIClicked|IsClicked(Message) _hitactor X 0.0))

(event Custom|Hold
  (params (X :type Float%20%28single-precision%29) (Y :type Float%20%28single-precision%29))
  (bind _returnvalue (Game|GetPlayerController 0))
  (bind _array (Utilities|Array|MakeArray "ObjectTypeQuery2"))
  (bind _hitresult (Class|PlayerController|GetHitResultUnderCursorforObjects _returnvalue _array true))
  (bind (_bblockinghit _binitialoverlap _time _distance _location _impactpoint _normal _impactnormal _physmat _hitactor) (Collision|BreakHitResult _hitresult))
  (if _bblockinghit
    (bind _output_get (Variables|Default|SetTraceObject _hitactor))
    (Timeline|Timeline_0 PlayFromStart
      (:Update
        (Class|BPIClicked|IsClickHold(Message) _output_get (Variables|Default|GetHoldX) 0.0)))))

(event Custom|Release
  (params (X :type Float%20%28single-precision%29) (Y :type Float%20%28single-precision%29))
  (Class|BPIClicked|IsReleased(Message) (Variables|Default|GetTraceObject) X 0.0)
  (Timeline|Timeline_0 Stop
    (:Update
      (Class|BPIClicked|IsClickHold(Message) (stale Custom|Hold _output_get) (Variables|Default|GetHoldX) 0.0))))

(event EventBeginPlay
  (Input|EnableInput (Game|GetPlayerController 0)))

(event Input|TouchEvents|InputTouch
  (params (Location :type Vector) (FingerIndex :type ETouchIndex%20Enum))
  (:Pressed
    (Utilities|MHold 0.1 :!label _label
      (:Tap
        (CallFunction|Click (.x Location) 0.0))
      (:Hold
        (CallFunction|Hold 0.0 0.0))
      (:Release
        (CallFunction|Release (.x Location) 0.0))))
  (:Released
    (goto _label Released))
  (:Moved
    (Variables|Default|SetHoldX (.x Location))))

(fn ConstructionScript)

(fn OnTouch
  (params (NewParam :type Pointer%20Event%20Structure))
  (Development|PrintString (Utilities|String|ToString(Float) (.x (Class|KismetInputLibrary|PointerEventGetScreenSpacePosition NewParam))))
  (return))