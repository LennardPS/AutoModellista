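; BP_RaceManager is a race manager actor that runs a running lap timer and prints it on screen.
; Tick uses a 0.1-second Delay as a throttle to count tenths into seconds, then prints the time every frame.
; The 60-second rollover branch is empty, and StartLap only prints "Start" without touching the timer.
; BeginPlay caches a BP_Car reference, which the shown graphs never use.
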(event EventStartLap
  (Development|PrintString "Start"))

(event EventTick
  (params (DeltaSeconds :type Float%20%28single-precision%29))
  (Variables|Default|SetDelta%20Seconds DeltaSeconds)
  (Utilities|FlowControl|Sequence
    (:then_0
      ;[1 1 1] LapTime
      (Utilities|FlowControl|Delay 0.1)
      (Variables|Default|SetTenthsOfSeconds (+ (Variables|Default|GetTenthsOfSeconds) 1))
      (if (>= (Variables|Default|GetTenthsOfSeconds) 10)
        (Variables|Default|SetTenthsOfSeconds 0)
        (Variables|Default|SetSeconds (+ (Variables|Default|GetSeconds) 1))
        (if (>= (Variables|Default|GetSeconds) 60)
          _)))
    (:then_3
      (Development|PrintString (Utilities|String|Append (Utilities|String|Append (Utilities|String|ToString(Integer) (Variables|Default|GetSeconds)) ".") (Utilities|String|ToString(Integer) (Variables|Default|GetTenthsOfSeconds))) true true "(R=1.000000,G=0.000000,B=0.726994,A=1.000000)" (Variables|Default|GetDelta%20Seconds)))))

(event EventBeginPlay
  (bind _returnvalue (Actor|GetActorOfClass "/Game/CarPawn/BP_Car.BP_Car_C"))
  (Variables|Default|SetCarRef _returnvalue))

(fn ConstructionScript)